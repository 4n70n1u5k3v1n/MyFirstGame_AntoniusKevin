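; BP_BaseItem is a configurable item actor that shows proximity icons as the player approaches.
; Entering OuterSphere shows the outer icon, and entering InnerSphere swaps it for the inner icon, with end overlaps reversing each step.
; Only the first player's character triggers the icons.
; The construction script applies sphere radii, mesh, scale and relative offset from variables, and shows both icons when IsDebugging is set.
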(event `self.InnerSphere.OnComponentBeginOverlap`
  (params (OverlappedComponent :type "PrimitiveComponent Object Reference") (OtherActor :type "Actor Object Reference") (OtherComp :type "PrimitiveComponent Object Reference") (OtherBodyIndex :type Integer) (bFromSweep :type Boolean) (SweepResult :type "HitResult Structure (by ref)"))
  (if (== OtherActor (`GameplayStatics.GetPlayerCharacter` 0))
    (`SceneComponent.SetVisibility` (`self.InnerSphereIcon`) true false)
    (`SceneComponent.SetVisibility` (`self.OuterSphereIcon`) false false)))

(event `self.InnerSphere.OnComponentEndOverlap`
  (params (OverlappedComponent :type "PrimitiveComponent Object Reference") (OtherActor :type "Actor Object Reference") (OtherComp :type "PrimitiveComponent Object Reference") (OtherBodyIndex :type Integer))
  (if (== (`GameplayStatics.GetPlayerCharacter` 0) OtherActor)
    (`SceneComponent.SetVisibility` (`self.InnerSphereIcon`) false false)
    (`SceneComponent.SetVisibility` (`self.OuterSphereIcon`) true false)))

(event `self.OuterSphere.OnComponentBeginOverlap`
  (params (OverlappedComponent :type "PrimitiveComponent Object Reference") (OtherActor :type "Actor Object Reference") (OtherComp :type "PrimitiveComponent Object Reference") (OtherBodyIndex :type Integer) (bFromSweep :type Boolean) (SweepResult :type "HitResult Structure (by ref)"))
  (if (== OtherActor (`GameplayStatics.GetPlayerCharacter` 0))
    (`SceneComponent.SetVisibility` (`self.OuterSphereIcon`) true false)))

(event `self.OuterSphere.OnComponentEndOverlap`
  (params (OverlappedComponent :type "PrimitiveComponent Object Reference") (OtherActor :type "Actor Object Reference") (OtherComp :type "PrimitiveComponent Object Reference") (OtherBodyIndex :type Integer))
  (if (== (`GameplayStatics.GetPlayerCharacter` 0) OtherActor)
    (`SceneComponent.SetVisibility` (`self.OuterSphereIcon`) false false)))

(fn `UserConstructionScript`
  (bind _staticmesh (`self.StaticMesh`))
  (`|ExecutionSequence`
    (:`then_0`
      (`SphereComponent.SetSphereRadius` (`self.InnerSphere`) (`self.InnerSphereRadius`) true)
      (`SphereComponent.SetSphereRadius` (`self.OuterSphere`) (`self.OuterSphereRadius`) true))
    (:`then_1`
      (`StaticMeshComponent.SetStaticMesh` _staticmesh (`self.NewMesh`))
      (`SceneComponent.K2_SetWorldTransform` _staticmesh (`KismetMathLibrary.MakeTransform` (`SceneComponent.K2_GetComponentLocation` _staticmesh) (`SceneComponent.K2_GetComponentRotation` _staticmesh) (`self.NewTransformScale`)) false false))
    (:`then_2`
      (`SceneComponent.K2_SetRelativeLocation` (`self.StaticMesh`) (`self.NewLocation`) false false))
    (:`then_3`
      (if (`self.IsDebugging`)
        (`SceneComponent.SetVisibility` (`self.InnerSphereIcon`) true false)
        (`SceneComponent.SetVisibility` (`self.OuterSphereIcon`) true false)))))