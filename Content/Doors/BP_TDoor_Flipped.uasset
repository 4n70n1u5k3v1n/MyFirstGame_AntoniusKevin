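; BP_TDoor_Flipped is an interactable door that toggles open and closed, swinging to a negative yaw.
; Interact flips IsOpened and plays or reverses the TL_Door timeline, whose curve drives a lerp on SMDoor's relative rotation.
; An IsOpening flag blocks further interaction until the timeline finishes.
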(event `self.Interact`
  ;[1 1 1] Door Toggle
  (if (not (`self.IsOpening`))
    (set `self.IsOpening` true)
    (if (`self.IsOpened`)
      (set `self.IsOpened` false)
      (bind (_direction _door) (`Timeline|TL_Door` :!via `Reverse` :!label _label)
        (:`Update`
          (`SceneComponent.K2_SetRelativeRotation` (`self.SM_Door`) (`KismetMathLibrary.MakeRotator` 0.0 0.0 (`KismetMathLibrary.Lerp` 0.0 -100.0 _door)) false false))
        (:`Finished`
          (set `self.IsOpening` false)))
      (else
        (set `self.IsOpened` true)
        (goto _label)))))

(fn `UserConstructionScript`)