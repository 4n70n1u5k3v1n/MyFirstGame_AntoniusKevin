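; Item inspection actor that shows a given mesh through a scene capture with a name and description widget, taking input away from the character.
; Callers supply the mesh, text, rotation and scale through its Inspect and setter events.
; Left-drag rotates the mesh, right-click restores the initial rotation and default zoom, and the wheel zooms via clamped capture FOV.
; The Interact input returns control to the character, removes the widget and destroys the actor.
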(event `/Game/FirstPerson/Blueprints/Interface/I_Interact.Inspect`
  (params (Character :type "/Game/FirstPerson/Blueprints/BP_FirstPersonCharacter Object Reference") (InspectedItem :type "StaticMesh Object Reference") (ItemName :type Text) (ItemDescription :type Text))
  (bind _returnvalue (`GameplayStatics.GetPlayerController` 0))
  (set `self.Character` Character)
  (`StaticMeshComponent.SetStaticMesh` (`self.InspectedItem`) InspectedItem)
  (bind _returnvalue_2 (`|CreateWidget` "/Game/Widget/WBP_Inspection.WBP_Inspection_C" null ItemName ItemDescription))
  (bind _output_get (set `self.WBP_Inspect` _returnvalue_2))
  (`UserWidget.AddToViewport` _output_get 0)
  (`self.DisableInput` (`self.Character`) _returnvalue)
  (`self.EnableInput` _returnvalue))

(event `EnhancedInput|/Game/FirstPerson/Input/Actions/IA_Interact`
  (params (ActionValue :type Boolean) (ElapsedSeconds :type "Float (double-precision)") (TriggeredSeconds :type "Float (double-precision)") (InputAction :type "InputAction Object Reference" :default "/Game/FirstPerson/Input/Actions/IA_Interact.IA_Interact"))
  (bind _returnvalue (`GameplayStatics.GetPlayerController` 0))
  (bind _wbp_inspect (`self.WBP_Inspect`))
  (:`Triggered`
    (`self.DisableInput` _returnvalue)
    (`self.EnableInput` (`self.Character`) _returnvalue)
    (`/Engine/EditorBlueprintResources/StandardMacros.IsValid` _wbp_inspect
      (:`Is Valid`
        (`Widget.RemoveFromParent` _wbp_inspect)
        (set `self.WBP_Inspect` null)
        (`self.K2_DestroyActor`)))))

(event `SetItemRotation`
  (params (ItemRotation :type "Rotator Structure"))
  (bind _inspecteditem (`self.InspectedItem`))
  (bind (_returnvalue_location _returnvalue_rotation _returnvalue_scale) (`KismetMathLibrary.BreakTransform` (`SceneComponent.K2_GetComponentToWorld` _inspecteditem)))
  (set `self.InitialRotation` ItemRotation)
  (`SceneComponent.K2_SetWorldTransform` _inspecteditem (`KismetMathLibrary.MakeTransform` _returnvalue_location ItemRotation _returnvalue_scale) false false))

(event `SetItemScale`
  (params (ItemScale :type "Vector Structure (by ref)"))
  (bind _inspecteditem (`self.InspectedItem`))
  (bind (_returnvalue_location _returnvalue_rotation) (`KismetMathLibrary.BreakTransform` (`SceneComponent.K2_GetComponentToWorld` _inspecteditem)))
  (`SceneComponent.K2_SetWorldTransform` _inspecteditem (`KismetMathLibrary.MakeTransform` _returnvalue_location _returnvalue_rotation ItemScale) false false))

(event `Key|LeftMouseButton`
  (params (Key :type "Key Structure"))
  (:`Pressed`
    (set `self.IsRotating` true))
  (:`Released`
    (set `self.IsRotating` false)))

(event `Key|RightMouseButton`
  (params (Key :type "Key Structure"))
  (:`Pressed`
    (`SceneComponent.K2_SetWorldRotation` (`self.InspectedItem`) (`self.InitialRotation`) false false)
    (set `SceneCaptureComponent2D.FOVAngle` 50.0 (`self.SceneCaptureComponent2D`))))

(event `InputAxisKey|MouseX`
  (params (AxisValue :type "Float (single-precision)"))
  (bind _inspecteditem (`self.InspectedItem`))
  (if (`self.IsRotating`)
    (`SceneComponent.K2_SetWorldRotation` _inspecteditem (`KismetMathLibrary.ComposeRotators` (`SceneComponent.K2_GetComponentRotation` _inspecteditem) (`KismetMathLibrary.MakeRotator` 0.0 0.0 (* AxisValue -3.0))) false false)))

(event `InputAxisKey|MouseY`
  (params (AxisValue :type "Float (single-precision)"))
  (bind _inspecteditem (`self.InspectedItem`))
  (if (`self.IsRotating`)
    (`SceneComponent.K2_SetWorldRotation` _inspecteditem (`KismetMathLibrary.ComposeRotators` (`SceneComponent.K2_GetComponentRotation` _inspecteditem) (`KismetMathLibrary.MakeRotator` 0.0 (* AxisValue -3.0))) false false)))

(event `Key|MouseScrollUp`
  (params (Key :type "Key Structure"))
  (bind _scenecapturecomponent2d (`self.SceneCaptureComponent2D`))
  (:`Pressed`
    (set `SceneCaptureComponent2D.FOVAngle` (`KismetMathLibrary.FClamp` (- (`SceneCaptureComponent2D.FOVAngle` _scenecapturecomponent2d) 1.0) 30.0 90.0) _scenecapturecomponent2d)))

(event `Key|MouseScrollDown`
  (params (Key :type "Key Structure"))
  (bind _scenecapturecomponent2d (`self.SceneCaptureComponent2D`))
  (:`Pressed`
    (set `SceneCaptureComponent2D.FOVAngle` (`KismetMathLibrary.FClamp` (+ (`SceneCaptureComponent2D.FOVAngle` _scenecapturecomponent2d) 1.0) 30.0 90.0) _scenecapturecomponent2d)))

(fn `UserConstructionScript`)