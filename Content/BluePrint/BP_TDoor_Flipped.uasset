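; BP_TDoor_Flipped is an interactable swinging door that can start locked and unlocks when PickupKeyItem fires.
; Interact plays or reverses a timeline that lerps the door mesh's yaw to open toward negative yaw, ignoring input while moving.
; Nested inner and outer overlap spheres swap two pairs of icons as the player approaches, showing outer icons at range and inner icons up close.
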(event `self.Interact`
  (params (Character :type "/Game/FirstPerson/Blueprints/BP_FirstPersonCharacter Object Reference"))
  ;[1 1 1] Door Toggle
  (if (`self.IsLocked`)
    _
    (elif (not (`self.IsOpening`))
      (set `self.IsOpening` true)
      (if (`self.IsOpened`)
        (set `self.IsOpened` false)
        (bind (_direction _door) (`Timeline|TL_Door` :!via `Reverse` :!label _label)
          (:`Update`
            (`SceneComponent.K2_SetRelativeRotation` (`self.SM_Door`) (`KismetMathLibrary.MakeRotator` 0.0 0.0 (`KismetMathLibrary.Lerp` 0.0 -100.0 _door)) false false))
          (:`Finished`
            (set `self.IsOpening` false)))
        (else
          (set `self.IsOpened` true)
          (goto _label))))))

(event `self.InnerSphere.OnComponentBeginOverlap`
  (params (OverlappedComponent :type "PrimitiveComponent Object Reference") (OtherActor :type "Actor Object Reference") (OtherComp :type "PrimitiveComponent Object Reference") (OtherBodyIndex :type Integer) (bFromSweep :type Boolean) (SweepResult :type "HitResult Structure (by ref)"))
  (if (== OtherActor (`GameplayStatics.GetPlayerCharacter` 0))
    (`SceneComponent.SetVisibility` (`self.InnerSphereIcon1`) true false)
    (`SceneComponent.SetVisibility` (`self.InnerSphereIcon2`) true false)
    (`SceneComponent.SetVisibility` (`self.OuterSphereIcon1`) false false)
    (`SceneComponent.SetVisibility` (`self.OuterSphereIcon2`) false false)))

(event `self.InnerSphere.OnComponentEndOverlap`
  (params (OverlappedComponent :type "PrimitiveComponent Object Reference") (OtherActor :type "Actor Object Reference") (OtherComp :type "PrimitiveComponent Object Reference") (OtherBodyIndex :type Integer))
  (if (== (`GameplayStatics.GetPlayerCharacter` 0) OtherActor)
    (`SceneComponent.SetVisibility` (`self.InnerSphereIcon1`) false false)
    (`SceneComponent.SetVisibility` (`self.InnerSphereIcon2`) false false)
    (`SceneComponent.SetVisibility` (`self.OuterSphereIcon1`) true false)
    (`SceneComponent.SetVisibility` (`self.OuterSphereIcon2`) true false)))

(event `self.OuterSphere.OnComponentBeginOverlap`
  (params (OverlappedComponent :type "PrimitiveComponent Object Reference") (OtherActor :type "Actor Object Reference") (OtherComp :type "PrimitiveComponent Object Reference") (OtherBodyIndex :type Integer) (bFromSweep :type Boolean) (SweepResult :type "HitResult Structure (by ref)"))
  (if (== OtherActor (`GameplayStatics.GetPlayerCharacter` 0))
    (`SceneComponent.SetVisibility` (`self.OuterSphereIcon1`) true false)
    (`SceneComponent.SetVisibility` (`self.OuterSphereIcon2`) true false)))

(event `self.OuterSphere.OnComponentEndOverlap`
  (params (OverlappedComponent :type "PrimitiveComponent Object Reference") (OtherActor :type "Actor Object Reference") (OtherComp :type "PrimitiveComponent Object Reference") (OtherBodyIndex :type Integer))
  (if (== OtherActor (`GameplayStatics.GetPlayerCharacter` 0))
    (`SceneComponent.SetVisibility` (`self.OuterSphereIcon2`) false false)
    (`SceneComponent.SetVisibility` (`self.OuterSphereIcon1`) false false)))

(event `/Game/FirstPerson/Blueprints/Interface/I_Interact.Pickup Key Item`
  (params (Door :type "/Game/BluePrint/BP_TDoor Object Reference") (`Door Flipped` :type "/Game/BluePrint/BP_TDoor_Flipped Object Reference"))
  (set `self.IsLocked` false))

(fn `UserConstructionScript`)