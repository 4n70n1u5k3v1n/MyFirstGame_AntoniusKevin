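; BP_BaseItem is a base interactable world item that shows proximity icons and can open an inspection view.
; Nested inner and outer spheres toggle their icons as the player character enters and leaves.
; On Interact, inspectable items spawn a BP_InspectionItem at a far-off location, passing it mesh, text, display transform, pickup flag and level sequence data.
; The construction script configures mesh, sphere radii and icon placement, with a debug option revealing both icons.
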(event `self.InnerSphere.OnComponentBeginOverlap`
  (params (OverlappedComponent :type "PrimitiveComponent Object Reference") (OtherActor :type "Actor Object Reference") (OtherComp :type "PrimitiveComponent Object Reference") (OtherBodyIndex :type Integer) (bFromSweep :type Boolean) (SweepResult :type "HitResult Structure (by ref)"))
  (if (== OtherActor (`GameplayStatics.GetPlayerCharacter` 0))
    (`SceneComponent.SetVisibility` (`self.InnerSphereIcon`) true false)
    (`SceneComponent.SetVisibility` (`self.OuterSphereIcon`) false false)))

(event `self.InnerSphere.OnComponentEndOverlap`
  (params (OverlappedComponent :type "PrimitiveComponent Object Reference") (OtherActor :type "Actor Object Reference") (OtherComp :type "PrimitiveComponent Object Reference") (OtherBodyIndex :type Integer))
  (if (== (`GameplayStatics.GetPlayerCharacter` 0) OtherActor)
    (`SceneComponent.SetVisibility` (`self.InnerSphereIcon`) false false)
    (`SceneComponent.SetVisibility` (`self.OuterSphereIcon`) true false)))

(event `self.OuterSphere.OnComponentBeginOverlap`
  (params (OverlappedComponent :type "PrimitiveComponent Object Reference") (OtherActor :type "Actor Object Reference") (OtherComp :type "PrimitiveComponent Object Reference") (OtherBodyIndex :type Integer) (bFromSweep :type Boolean) (SweepResult :type "HitResult Structure (by ref)"))
  (if (== OtherActor (`GameplayStatics.GetPlayerCharacter` 0))
    (`SceneComponent.SetVisibility` (`self.OuterSphereIcon`) true false)))

(event `self.OuterSphere.OnComponentEndOverlap`
  (params (OverlappedComponent :type "PrimitiveComponent Object Reference") (OtherActor :type "Actor Object Reference") (OtherComp :type "PrimitiveComponent Object Reference") (OtherBodyIndex :type Integer))
  (if (== (`GameplayStatics.GetPlayerCharacter` 0) OtherActor)
    (`SceneComponent.SetVisibility` (`self.OuterSphereIcon`) false false)))

(event `/Game/FirstPerson/Blueprints/Interface/I_Interact.Interact`
  (params (Character :type "/Game/FirstPerson/Blueprints/BP_FirstPersonCharacter Object Reference"))
  (if (`self.IsInspectable`)
    (bind _returnvalue (`|SpawnActorFromClass` "/Game/BluePrint/BP_InspectionItem.BP_InspectionItem_C" (`KismetMathLibrary.MakeTransform` (10000000.0 0.0 0.0)) "Undefined" "MultiplyWithRoot" null null))
    (`/Game/BluePrint/BP_InspectionItem.SetItemRotation` _returnvalue (`self.InspectItemRotation`))
    (`/Game/BluePrint/BP_InspectionItem.SetItemScale` _returnvalue (`self.InspectItemScale`))
    (`/Game/FirstPerson/Blueprints/Interface/I_Interact.Inspect` _returnvalue Character (`StaticMeshComponent.StaticMesh` (`self.StaticMesh`)) (`self.ItemName`) (`self.ItemDescription`) (`self.IsPickupable`) self (`self.HasLevelSequence`) (`self.LevelSequenceActor`))))

(fn `UserConstructionScript`
  (bind _staticmesh (`self.StaticMesh`))
  (`|ExecutionSequence`
    (:`then_0`
      (`SphereComponent.SetSphereRadius` (`self.InnerSphere`) (`self.InnerSphereRadius`) true)
      (`SphereComponent.SetSphereRadius` (`self.OuterSphere`) (`self.OuterSphereRadius`) true))
    (:`then_1`
      (`StaticMeshComponent.SetStaticMesh` _staticmesh (`self.NewStaticMesh`))
      (`SceneComponent.K2_SetWorldTransform` _staticmesh (`KismetMathLibrary.MakeTransform` (`SceneComponent.K2_GetComponentLocation` _staticmesh) (`SceneComponent.K2_GetComponentRotation` _staticmesh) (`self.NewTransformScale`)) false false)
      (`PrimitiveComponent.SetMaterial` (`self.StaticMesh`) 0 null))
    (:`then_2`
      (`SceneComponent.K2_SetRelativeLocation` (`self.StaticMesh`) (`self.NewStaticMeshLocation`) false false))
    (:`then_3`
      (`SceneComponent.K2_SetRelativeLocation` (`self.OuterSphereIcon`) (`self.NewIconLocation`) false false)
      (`SceneComponent.K2_SetRelativeLocation` (`self.InnerSphereIcon`) (`self.NewIconLocation`) false false))
    (:`then_4`
      (if (`self.IsDebugging`)
        (`SceneComponent.SetVisibility` (`self.InnerSphereIcon`) true false)
        (`SceneComponent.SetVisibility` (`self.OuterSphereIcon`) true false)))
    (:`then_5`
      (`SphereComponent.SetSphereRadius` (`self.CollisionSphere`) (`self.In Sphere Radius`) true))))