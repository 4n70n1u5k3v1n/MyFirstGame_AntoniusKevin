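; BP_LightSwitch is an interactable switch that turns a set of lights on and off.
; Its Interact event loops over the Lights array and sets each light component's intensity to zero or a fixed brightness, based on the IsOn flag.
; It then flips IsOn, so each interaction toggles the whole group together.
; The construction script only calls its parent.
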(event `/Game/FirstPerson/Blueprints/Interface/I_Interact.Interact`
  (params (Character :type "/Game/FirstPerson/Blueprints/BP_FirstPersonCharacter Object Reference"))
  (for _array_element (`self.Lights`)
    (if (`self.IsOn`)
      (bind _lightcomponent (`Light.LightComponent` _array_element))
      (`LightComponent.SetIntensity` _lightcomponent 0.0)
      (else
        (`LightComponent.SetIntensity` _lightcomponent 6.0))))
  (if (`self.IsOn`)
    (set `self.IsOn` false)
    (else
      (set `self.IsOn` true))))

(fn `UserConstructionScript`
  (`parent.UserConstructionScript`))