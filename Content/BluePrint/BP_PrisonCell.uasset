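; BP_PrisonCell is an interactable prison cell that gives way to a separate broken version when breakable.
; On Interact, if IsBreakable is set, it applies DeltaTransform to the referenced BrokenPrisonCell's root as an additive, teleporting world offset, then destroys itself.
; The broken cell is moved rather than spawned, and the construction script does nothing.
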(event `/Game/FirstPerson/Blueprints/Interface/I_Interact.Interact`
  (params (Character :type "/Game/FirstPerson/Blueprints/BP_FirstPersonCharacter Object Reference"))
  (if (`self.IsBreakable`)
    (`SceneComponent.K2_AddWorldTransform` (`Actor.RootComponent` (`self.BrokenPrisonCell`)) (`self.Delta Transform`) false true)
    (`self.K2_DestroyActor`)))

(fn `UserConstructionScript`)