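; BP_Drawer is an interactable drawer that moves its static mesh when Interact fires.
; Each interaction updates the stored DeltaX, DeltaY and DeltaZ values, then applies them as a world-space location offset.
; The move is a single teleport step, with no timeline or interpolation.
; The construction script only calls its parent.
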(event `/Game/FirstPerson/Blueprints/Interface/I_Interact.Interact`
  (params (Character :type "/Game/FirstPerson/Blueprints/BP_FirstPersonCharacter Object Reference"))
  (bind _result (`/Engine/EditorBlueprintResources/StandardMacros.NegateFloat` (`self.Delta  X`))
    (:`  `
      (set `self.Delta  X` _result)
      (bind _result_2 (`/Engine/EditorBlueprintResources/StandardMacros.NegateFloat` (`self.Delta Y`))
        (:`  `
          (set `self.Delta Y` _result_2)
          (bind _result_3 (`/Engine/EditorBlueprintResources/StandardMacros.NegateFloat` (`self.Delta Z`))
            (:`  `
              (set `self.Delta Z` _result_3)
              (`SceneComponent.K2_AddWorldTransform` (`self.StaticMesh`) (`KismetMathLibrary.MakeTransform` (`KismetMathLibrary.MakeVector` (`self.Delta  X`) (`self.Delta Y`) (`self.Delta Z`))) false true))))))))

(fn `UserConstructionScript`
  (`parent.UserConstructionScript`))